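; Dialogue component for the Psychic NPC, running a short branching conversation about the player's relationship to an unnamed woman.
; The overridden Dialogue function asks one question with three options, each leading to a single reply from the Psychic.
; Every branch then clears dialogue progress and closes the conversation, so the choice is not saved.
; Unconnected template nodes remain for branch-based progress saving.
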(fn `Dialogue`
  (`parent.Dialogue`)
  (switch `int` 0
    (:`0`
      (bind (_state _optionindex) (`self.AddDialogue` "Psychic" "What was she to you?" (`|MakeArray` "She was my friend." "She was more." "I don't need to answer this." :!type "Text")))
      (switch `/Game/Blackwood/Dialogue/Blueprints/Enum_DialogueState` _state
        (:`NewEnumerator0`
          (switch `int` _optionindex
            (:`0`
              (bind _state_2 (`self.AddDialogue` "Psychic" "Are you sure?" (`|MakeArray`)))
              (switch `/Game/Blackwood/Dialogue/Blueprints/Enum_DialogueState` _state_2
                (:`NewEnumerator0`
                  (`self.ClearDialogueProgress`)
                  (`self.CloseConversation`))))
            (:`1`
              (bind _state_3 (`self.AddDialogue` "Psychic" "You meant more to her as well." (`|MakeArray`)))
              (switch `/Game/Blackwood/Dialogue/Blueprints/Enum_DialogueState` _state_3
                (:`NewEnumerator0`
                  (`self.ClearDialogueProgress`)
                  (`self.CloseConversation`))))
            (:`2`
              (bind _state_4 (`self.AddDialogue` "Psychic" "No. But it might help." (`|MakeArray`)))
              (switch `/Game/Blackwood/Dialogue/Blueprints/Enum_DialogueState` _state_4
                (:`NewEnumerator0`
                  (`self.ClearDialogueProgress`)
                  (`self.CloseConversation`))))))))))